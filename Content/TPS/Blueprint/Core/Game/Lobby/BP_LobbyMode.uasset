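; Multiplayer lobby game mode that seats joining players, manages their colors and server-travels to the selected level.
; PostLogin spawns a lobby character at a free TargetPoint, tracked in an occupancy map, and assigns a random available color.
; Color changes and logouts update blocked colors in BP_LobbyGameState, with logout also freeing the spawn point.
; It pushes level selection to each controller and can save colors by player name in the GameInstance.
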(event `UpdateLevelName`
  (params (SlecetedLevel :type Name))
  (set `self.SelectedLevel` SlecetedLevel)
  (for _array_element (`self.PlayerControllers`)
    (bind _asbp_lobby_player_controller (cast `/Game/TPS/Blueprint/Core/Game/Lobby/BP_LobbyPlayerController` _array_element))
    (`/Game/TPS/Blueprint/Core/Game/Lobby/BP_LobbyPlayerController.UpdateLobbyWidget_OnClient` _asbp_lobby_player_controller (`self.SelectedLevel`))))

(event `LaunchGame`
  (`KismetSystemLibrary.ExecuteConsoleCommand` (`KismetStringLibrary.Concat_StrStr` "servertravel " (`KismetStringLibrary.Conv_NameToString` (`self.SelectedLevel`))) (`GameplayStatics.GetPlayerController` 0)))

(event `self.K2_PostLogin`
  (params (NewPlayer :type "PlayerController Object Reference"))
  (bind _targetpoint (`self.TargetPoint`))
  (bind _keys (`BlueprintMapLibrary.Map_Keys` (`self.TargetPoint`)))
  (if (not (> (`KismetArrayLibrary.Array_Length` _keys) 0))
    (bind _outactors (`GameplayStatics.GetAllActorsOfClass` "/Script/Engine.TargetPoint"))
    (for _array_element _outactors
      (`BlueprintMapLibrary.Map_Add` (`self.TargetPoint`) _array_element)))
  (`KismetArrayLibrary.Array_Add` (`self.PlayerControllers`) NewPlayer)
  (bind _keys_2 (`BlueprintMapLibrary.Map_Keys` _targetpoint))
  (for _array_element_2 _keys_2
    (if (not (`BlueprintMapLibrary.Map_Find` _targetpoint _array_element_2))
      (`BlueprintMapLibrary.Map_Add` _targetpoint _array_element_2 true)
      (bind _returnvalue (`|SpawnActorFromClass` "/Game/TPS/Blueprint/Core/Game/Lobby/BP_LobbyCharacter.BP_LobbyCharacter_C" (`self.GetTransform` _array_element_2) "Undefined" "OverrideRootScale" null null))
      (bind _asbp_lobby_player_controller (cast `/Game/TPS/Blueprint/Core/Game/Lobby/BP_LobbyPlayerController` NewPlayer))
      (set `/Game/TPS/Blueprint/Core/Game/Lobby/BP_LobbyPlayerController.OccupiedPoint` _array_element_2 _asbp_lobby_player_controller)
      (`/Game/TPS/Blueprint/Core/Game/Lobby/BP_LobbyPlayerController.SaveLobbyCharacter` _asbp_lobby_player_controller _returnvalue)
      (set `/Game/TPS/Blueprint/Core/Game/Lobby/BP_LobbyPlayerController.CurrentLevelByServer` (`self.SelectedLevel`) _asbp_lobby_player_controller)
      (`self.SetRandomlyColorCharAndUpdateColorState` _asbp_lobby_player_controller)
      (break))))

(event `self.K2_OnLogout`
  (params (ExitingController :type "Controller Object Reference"))
  (bind _asbp_lobby_player_controller (cast `/Game/TPS/Blueprint/Core/Game/Lobby/BP_LobbyPlayerController` ExitingController))
  (`KismetArrayLibrary.Array_RemoveItem` (`self.PlayerControllers`) _asbp_lobby_player_controller)
  (`BlueprintMapLibrary.Map_Add` (`self.TargetPoint`) (`/Game/TPS/Blueprint/Core/Game/Lobby/BP_LobbyPlayerController.OccupiedPoint` _asbp_lobby_player_controller) false)
  (bind _asbp_lobby_game_state (cast `/Game/TPS/Blueprint/Core/Game/Lobby/BP_LobbyGameState` (`GameplayStatics.GetGameState`)))
  (`/Game/TPS/Blueprint/Core/Game/Lobby/BP_LobbyGameState.AddOrRemoveColorToBlock_OnServer` _asbp_lobby_game_state (`/Game/TPS/Blueprint/Core/Game/Lobby/BP_LobbyCharacter.CurrentColor` (`/Game/TPS/Blueprint/Core/Game/Lobby/BP_LobbyPlayerController.LobbyCharacter` _asbp_lobby_player_controller)) true))

(event `UpdateColorForCharacter`
  (params (Color :type "MaterialInterface Object Reference") (Controller :type "/Game/TPS/Blueprint/Core/Game/Lobby/BP_LobbyPlayerController Object Reference"))
  (bind _asbp_lobby_game_state (cast `/Game/TPS/Blueprint/Core/Game/Lobby/BP_LobbyGameState` (`GameplayStatics.GetGameState`)))
  (`/Game/TPS/Blueprint/Core/Game/Lobby/BP_LobbyGameState.SelectedNewColor_OnServer` _asbp_lobby_game_state (`/Game/TPS/Blueprint/Core/Game/Lobby/BP_LobbyCharacter.CurrentColor` (`/Game/TPS/Blueprint/Core/Game/Lobby/BP_LobbyPlayerController.LobbyCharacter` Controller)) Color)
  (`/Game/TPS/Blueprint/Core/Game/Lobby/BP_LobbyPlayerController.UdpateLobbyCharacterParam` Controller Color))

(event `self.ReceiveTick`
  (params (DeltaSeconds :type "Float (single-precision)")))

(event `CustomEvent_0`)

(event `SaveColorForPlayers`
  (bind _asbp_game_instance (cast `/Game/TPS/Blueprint/Core/Game/BP_GameInstance` (`GameplayStatics.GetGameInstance`)))
  (for _array_element (`self.PlayerControllers`)
    (bind _asbp_lobby_player_controller (cast `/Game/TPS/Blueprint/Core/Game/Lobby/BP_LobbyPlayerController` _array_element))
    (`BlueprintMapLibrary.Map_Add` (`/Game/TPS/Blueprint/Core/Game/BP_GameInstance.ColorForPlayers` _asbp_game_instance) (`PlayerState.GetPlayerName` (`Controller.PlayerState` _array_element)) (`/Game/TPS/Blueprint/Core/Game/Lobby/BP_LobbyCharacter.CurrentColor` (`/Game/TPS/Blueprint/Core/Game/Lobby/BP_LobbyPlayerController.LobbyCharacter` _asbp_lobby_player_controller)))
    (`/Game/TPS/Blueprint/Core/Game/Lobby/BP_LobbyPlayerController.RemoveAllWidget` _asbp_lobby_player_controller)))

(fn `SetRandomlyColorCharAndUpdateColorState`
  (params (TargetController :type "/Game/TPS/Blueprint/Core/Game/Lobby/BP_LobbyPlayerController Object Reference"))
  (locals (SelectedColor :type "MaterialInterface Object Reference"))
  (bind _selectedcolor (`local.SelectedColor`))
  (bind _asbp_lobby_game_state (cast `/Game/TPS/Blueprint/Core/Game/Lobby/BP_LobbyGameState` (`GameplayStatics.GetGameState`)))
  (bind _aviablecolorout (`/Game/TPS/Blueprint/Core/Game/Lobby/BP_LobbyGameState.GetAviableColors` _asbp_lobby_game_state))
  (set `local.SelectedColor` (`|GetArrayItem` _aviablecolorout (`KismetMathLibrary.RandomInteger` (- (`KismetArrayLibrary.Array_Length` _aviablecolorout) 1))))
  (`/Game/TPS/Blueprint/Core/Game/Lobby/BP_LobbyGameState.AddOrRemoveColorToBlock_OnServer` _asbp_lobby_game_state _selectedcolor false)
  (`/Game/TPS/Blueprint/Core/Game/Lobby/BP_LobbyPlayerController.UdpateLobbyCharacterParam` TargetController _selectedcolor))

(fn `UserConstructionScript`)