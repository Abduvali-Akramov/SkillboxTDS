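; Base enemy character for the TPS game, handling health reactions, melee attacks, death and ammo-type loot.
; Damage feeds TPSHealth, whose change event spawns damage numbers and randomly triggers confusion stuns, hit animations or timed slowdowns applied on Tick.
; Light and heavy attack montages gate attack/movement flags and use notifies to sphere-trace damage against Player-tagged actors.
; Death unpossesses, drops any randomly added weapon-type pickup, then ragdolls after the death montage.
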(event `self.ReceiveTick`
  (params (DeltaSeconds :type "Float (single-precision)"))
  (set `self.DeltaTime` DeltaSeconds)
  (`self.ChangeSpeedByHit`))

(event `self.TPSHealth.OnHealthChange`
  (params (Health :type "Float (single-precision)") (Damage :type "Float (single-precision)"))
  (if (not (`self.bIsDead`))
    (if (> (`KismetMathLibrary.RandomFloat`) (`self.ConfusionChance`))
      (`self.ConfusionEnabledTimer`)
      (else
        (`self.HitAnim`)))
    (bind _returnvalue (`|SpawnActorFromClass` "/Game/TPS/Blueprint/InteractionEnvironment/DisplayDamage/BP_DisplayDamage.BP_DisplayDamage_C" (`KismetMathLibrary.MakeTransform` (+ (+ (`KismetMathLibrary.MakeVector` (`KismetMathLibrary.RandomFloatInRange` -20.0 20.0) (`KismetMathLibrary.RandomFloatInRange` -20.0 20.0)) (`self.SpawnOffsetLocalDamage`)) (`self.K2_GetActorLocation`))) "AlwaysSpawn" "OverrideRootScale" null null))
    (`/Game/TPS/Blueprint/InteractionEnvironment/DisplayDamage/BP_DisplayDamage.InitActor` _returnvalue Damage Health)
    (if (> (`KismetMathLibrary.RandomFloat`) (`self.SlowDownSpeedChance`))
      (set `self.SlowDownSpeed` true)
      (`KismetSystemLibrary.K2_SetTimerDelegate` (delegate `SlowDownDisabled`) 2.0))))

(event `SlowDownDisabled`
  (set `self.SlowDownSpeed` false))

(event `self.ReceiveAnyDamage`
  (params (Damage :type "Float (single-precision)") (DamageType :type "DamageType Object Reference") (InstigatedBy :type "Controller Object Reference") (DamageCauser :type "Actor Object Reference"))
  (`TPSHealthComponent.ChangeHealthValue` (`self.TPSHealth`) (* Damage -1.0)))

(event `self.TPSHealth.OnDead`
  (bind _deadsanim (`self.DeadsAnim`))
  (bind _output (`|GetArrayItem` _deadsanim (- (`KismetArrayLibrary.Array_Length` _deadsanim) 1)))
  (if (not (`self.bIsDead`))
    (`self.DeadEvent`)
    (`/Engine/EditorBlueprintResources/StandardMacros.IsValid` _output
      (:`Is Valid`
        (`|PlayMontage` (`self.Mesh`) _output
          (:`OnCompleted`
            (`PrimitiveComponent.SetCollisionProfileName` (`self.Mesh`) "PhysicsActor" true)
            (`PrimitiveComponent.SetCollisionEnabled` (`self.Mesh`) "PhysicsOnly")
            (`PrimitiveComponent.SetCollisionEnabled` (`self.Mesh`) "PhysicsOnly")
            (`PrimitiveComponent.SetCollisionResponseToChannel` (`self.CapsuleComponent`) "ECC_Pawn" "ECR_Ignore")
            (`PrimitiveComponent.SetCollisionResponseToChannel` (`self.Mesh`) "ECC_Pawn" "ECR_Ignore")
            (`PrimitiveComponent.SetSimulatePhysics` (`self.Mesh`) true)))))))

(event `self.ReceiveBeginPlay`
  (`self.InitDropComponent`))

(event `/Game/TPS/Blueprint/EnemyCharacter/Common/BPI_Combat.MeleeAttackLight`
  (bind _lightattackanim (`self.LightAttackAnim`))
  (bind _baselightdamage (`self.BaseLightDamage`))
  (`self.SetStateAttack` false)
  (bind _notifyname (`|PlayMontage` (`self.Mesh`) (`|GetArrayItem` _lightattackanim (`KismetMathLibrary.RandomInteger` (`KismetArrayLibrary.Array_Length` _lightattackanim))))
    (:`OnCompleted`
      (`self.SetStateAttack` true :!label _label))
    (:`OnInterrupted`
      (goto _label))
    (:`OnNotifyBegin`
      (if (== _notifyname "Attack")
        (`self.MeleeTrace` 50.0 150.0 (`KismetMathLibrary.RandomFloatInRange` (- _baselightdamage 10.0) (+ _baselightdamage 20.0)) (`self.LightRadius`))))))

(event `/Game/TPS/Blueprint/EnemyCharacter/Common/BPI_Combat.MeleeAttackHeavy`
  (bind _heavyattackanim (`self.HeavyAttackAnim`))
  (bind _baseheavydamage (`self.BaseHeavyDamage`))
  (`self.SetStateAttack` false)
  (`self.SetStateMovement` false)
  (bind _notifyname (`|PlayMontage` (`self.Mesh`) (`|GetArrayItem` _heavyattackanim (`KismetMathLibrary.RandomInteger` (`KismetArrayLibrary.Array_Length` _heavyattackanim))))
    (:`OnCompleted`
      (`self.SetStateMovement` true :!label _label_2)
      (goto _label))
    (:`OnInterrupted`
      (goto _label_2))
    (:`OnNotifyBegin`
      (if (== _notifyname "Attack")
        (`self.MeleeTrace` 50.0 (`self.EndHeavyTraceDistance`) (`KismetMathLibrary.RandomFloatInRange` (- _baseheavydamage 10.0) (+ _baseheavydamage 50.0)) (`self.HeavyRadius`))))))

(fn `CanAttack`
  (returns (isCanAttack :type Boolean))
  (return (`self.CanAttackPawn`)))

(fn `CanMove`
  (returns (bIsCanMove :type Boolean))
  (return (`self.CanMovePawn`)))

(fn `ConfusionDisabledTimer`
  (`self.SetStateMovement` true)
  (set `CharacterMovementComponent.MaxWalkSpeed` 400.0 (`self.CharacterMovement`)))

(fn `ConfusionEnabledTimer`
  (locals (CurrentMontage :type "AnimMontage Object Reference"))
  (bind _confusionanim (`self.ConfusionAnim`))
  (`self.SetStateMovement` false)
  (bind _output_get (set `local.CurrentMontage` (`|GetArrayItem` _confusionanim (`KismetMathLibrary.RandomIntegerInRange` 0 (- (`KismetArrayLibrary.Array_Length` _confusionanim) 1)))))
  (bind _returnvalue (`AnimSequenceBase.GetPlayLength` _output_get))
  (`KismetSystemLibrary.K2_SetTimer` null "ConfusionDisabledTimer" _returnvalue)
  (`self.PlayAnimMontage` (`local.CurrentMontage`))
  (set `CharacterMovementComponent.MaxWalkSpeed` 0.0 (`self.CharacterMovement`))
  (set `self.bIsConfused` true))

(fn `DeadEvent`
  (bind _dropcomponent (`self.DropComponent`))
  (`Controller.UnPossess` (`self.GetController`))
  (`self.SetLifeSpan` 20.0)
  (`self.SetStateAttack` false)
  (`self.SetStateMovement` false)
  (set `self.bIsDead` true)
  (`/Engine/EditorBlueprintResources/StandardMacros.IsValid` _dropcomponent
    (:`Is Valid`
      (`/Game/TPS/Blueprint/BP_DropItemComponent.Drop` _dropcomponent))))

(fn `HitAnim`
  (if (`self.bIsConfused`)
    _
    (elif (> (`KismetMathLibrary.RandomFloat`) (`self.HitAnimChance`))
      (`self.PlayAnimMontage` "/Game/TPS/Characters/EnemyZombie/Type2/Anim/zombie_reaction_hit__2__Montage.zombie_reaction_hit__2__Montage"))))

(fn `InitDropComponent`
  (locals (cout :type Integer))
  (if (> (`KismetMathLibrary.RandomFloat`) (`self.DropChance`))
    (bind _returnvalue (`AddComponent|NODE_AddBP_DropItemComponent-0`))
    (set `self.DropComponent` _returnvalue)
    (bind _output_get (set `/Game/TPS/Blueprint/BP_DropItemComponent.Type` (select `int` (`KismetMathLibrary.RandomIntegerInRange` 0 3) :`0` "RifleType" :`1` "ShotGunType" :`2` "SniperRifle" :`3` "GrenadeLauncher" :!type "EWeaponType Enum") _returnvalue))
    (`|ExecutionSequence`
      (:`then_0`
        (switch `EWeaponType` _output_get
          (:`RifleType`
            (set `local.cout` 30))
          (:`ShotGunType`
            (set `local.cout` 12))
          (:`SniperRifle`
            (set `local.cout` 6))
          (:`GrenadeLauncher`
            (set `local.cout` 2))))
      (:`then_1`
        (set `/Game/TPS/Blueprint/BP_DropItemComponent.Cout` (`local.cout`) _returnvalue)))))

(fn `SetStateAttack`
  (params (CanAttack :type Boolean))
  (set `self.CanAttackPawn` CanAttack))

(fn `SetStateMovement`
  (params (CanMove :type Boolean))
  (set `self.CanMovePawn` CanMove))

(fn `UserConstructionScript`)