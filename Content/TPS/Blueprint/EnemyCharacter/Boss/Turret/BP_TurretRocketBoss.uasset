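; BP_TurretRocketBoss is a boss turret that periodically fires missiles while its owning BP_CharacterEnemy_Boss is alive.
; A looping timer calls FireRocket, which checks the owner's TPSHealth and clears the timer once health is depleted.
; Each cycle plays the Shoot timeline, whose Shot event spawns a BP_MissleTurret just ahead of the Arrow and initializes it with inline mesh, trail, speed and radial explosion settings.
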(event `self.ReceiveBeginPlay`
  (bind _returnvalue (`KismetSystemLibrary.K2_SetTimerDelegate` (delegate `FireRocket`) 3.0 true))
  (set `self.FireRocket_HanldeTimer` _returnvalue))

(event `FireRocket`
  (bind _returnvalue (`self.GetOwner`))
  (bind _arrow (`self.Arrow`))
  (bind _asbp_character_enemy_boss (cast `/Game/TPS/Blueprint/EnemyCharacter/Boss/BP_CharacterEnemy_Boss` _returnvalue))
  (bind _returnvalue_2 (`TPSHealthComponent.GetCurrentHealth` (`/Game/TPS/Blueprint/EnemyCharacter/BP_CharacterEnemy_Base.TPSHealth` _asbp_character_enemy_boss)))
  (if (> _returnvalue_2 0.0)
    (`Timeline|Shoot` :!via `PlayFromStart`
      (:`Shot`
        (bind _returnvalue_3 (`|SpawnActorFromClass` "/Game/TPS/Blueprint/EnemyCharacter/Boss/Turret/BP_MissleTurret.BP_MissleTurret_C" (`KismetMathLibrary.MakeTransform` (+ (* (`SceneComponent.GetForwardVector` _arrow) 100.0) (`SceneComponent.K2_GetComponentLocation` _arrow)) (`SceneComponent.K2_GetComponentRotation` _arrow)) "AlwaysSpawn" "OverrideRootScale" _returnvalue null))
        (`ProjectileDefault.InitProjectile` _returnvalue_3 (make `ProjectileInfo` :`Projectile` "/Game/TPS/Blueprint/EnemyCharacter/Boss/Turret/BP_MissleTurret.BP_MissleTurret_C" :`ProjectileStaticMesh` "/Game/TPS/Characters/Boss/WeaponTurret_Boss/Missle/torpedo.torpedo" :`ProjectileStaticMeshOffset` (`KismetMathLibrary.MakeTransform` (0.0 0.0 0.0) (struct) (10.0 10.0 10.0)) :`ProjectileTrailFx` "/Game/TPS/Items/GameActor/Weapon/Weapon_RocketLauncher/FX/P_RocketLauncher_Trail_Dark.P_RocketLauncher_Trail_Dark" :`ProjectileTrailFxOffset` (`KismetMathLibrary.MakeTransform` (-30.0 0.0 0.0)) :`ProjectileDamage` 1.0 :`ProjectileInitSpeed` 500.0 :`ProjectileMaxSpeed` 1000.0 :`ExplodeFX` "/Game/TPS/Items/GameActor/Weapon/Weapon_RocketLauncher/FX/P_RocketLauncher_Explosion_Dark.P_RocketLauncher_Explosion_Dark" :`ExplodeSound` "/Game/TPS/Items/GameActor/Weapon/Weapon_RocketLauncher/Sound/RocketLauncher_Explosion_Cue.RocketLauncher_Explosion_Cue" :`ProjectileMaxRadiusDamage` 300.0 :`ProjectileMinRadiusDamage` 150.0 :`ExplodeMaxDamage` 30.0 :`ExplodeFalloffCoef` 2.0))))
    (else
      (`KismetSystemLibrary.K2_ClearAndInvalidateTimerHandle` (`self.FireRocket_HanldeTimer`)))))

(fn `UserConstructionScript`)