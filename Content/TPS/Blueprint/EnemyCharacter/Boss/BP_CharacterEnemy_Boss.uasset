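; BP_CharacterEnemy_Boss is the boss enemy character for the TPS game, equipped with a rocket turret.
; On BeginPlay it runs the parent logic, then spawns BP_TurretRocketBoss with itself as owner and snaps it to the mesh's RocketSocket.
; The turret is a separate actor, and this graph adds no other behavior: Tick is disabled and the construction script only calls the parent.
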(event `self.ReceiveBeginPlay`
  (bind _mesh (`self.Mesh`))
  (`parent.ReceiveBeginPlay`)
  (bind _returnvalue (`|SpawnActorFromClass` "/Game/TPS/Blueprint/EnemyCharacter/Boss/Turret/BP_TurretRocketBoss.BP_TurretRocketBoss_C" (`KismetMathLibrary.Conv_VectorToTransform` (`SceneComponent.GetSocketLocation` _mesh "RocketSocket")) "AlwaysSpawn" "OverrideRootScale" self null))
  (`SceneComponent.K2_AttachToComponent` (`Actor.RootComponent` _returnvalue) _mesh "RocketSocket" "SnapToTarget" "SnapToTarget" "SnapToTarget" true))

(fn `UserConstructionScript`
  (`parent.UserConstructionScript`))