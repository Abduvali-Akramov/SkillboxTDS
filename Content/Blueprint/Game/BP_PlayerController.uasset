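; Player controller that owns the in-game HUD and a slow-motion toggle.
; On BeginPlay it pushes a sound mix modifier, then creates the BPW_IngameWidget and adds it to the viewport.
; Possess initializes the widget's health bar and UnPossess unbinds it, both behind validity checks.
; Left Ctrl flip-flops global time dilation between slow motion and normal speed.
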(event `self.ReceiveBeginPlay`
  (`GameplayStatics.PushSoundMixModifier` null)
  (bind _returnvalue (`|CreateWidget` "/Game/Blueprint/Widget/BPW_IngameWidget.BPW_IngameWidget_C" self))
  (set `self.IngameWidget` _returnvalue)
  (`UserWidget.AddToViewport` _returnvalue 0))

(event `Key|LeftControl`
  (params (Key :type "Key Structure"))
  (:`Pressed`
    (`/Engine/EditorBlueprintResources/StandardMacros.FlipFlop`
      (:`A`
        (`GameplayStatics.SetGlobalTimeDilation` 0.1))
      (:`B`
        (`GameplayStatics.SetGlobalTimeDilation` 1.0)))))

(event `self.ReceiveUnPossess`
  (params (UnpossessedPawn :type "Pawn Object Reference"))
  (`/Engine/EditorBlueprintResources/StandardMacros.IsValid` null
    (:`Is Valid`
      (`/Game/Blueprint/Widget/Health/BPW_StatsCharacterBar.UnBindWidget` (`/Game/Blueprint/Widget/BPW_IngameWidget.HealthBar` (`self.IngameWidget`))))))

(event `self.ReceivePossess`
  (params (PossessedPawn :type "Pawn Object Reference"))
  (bind _ingamewidget (`self.IngameWidget`))
  (`/Engine/EditorBlueprintResources/StandardMacros.IsValid` _ingamewidget
    (:`Is Valid`
      (`/Game/Blueprint/Widget/Health/BPW_StatsCharacterBar.InitWidget` (`/Game/Blueprint/Widget/BPW_IngameWidget.HealthBar` _ingamewidget)))))

(fn `UserConstructionScript`)