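; Game mode that runs phase-based enemy spawning, player respawning and the win condition, with progress held in BP_GameState.
; A looping timer asks the game state whether to spawn, then places an enemy at a random current-phase spawn point or within its box.
; Player respawns use the phase's tagged start, and enemy deaths feed score that can trigger the end-game widget.
; Phase changes strip score components from living enemies.
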(event `self.ReceiveBeginPlay`
  (`KismetSystemLibrary.K2_SetTimer` null "TryRespawnEnemy" 1.0 true))

(fn `EnemyDead`
  (params (Score :type Integer))
  (if (> Score 0)
    (bind _asbp_game_state (cast `/Game/Blueprint/Game/BP_GameState` (`GameplayStatics.GetGameState`)))
    (bind _biswin (`/Game/Blueprint/Game/BP_GameState.Increment Score` _asbp_game_state Score))
    (`/Game/Blueprint/Game/BP_GameState.Increment Score` _asbp_game_state -1)
    (if _biswin
      (bind _returnvalue (`|CreateWidget` "/Game/Blueprint/Widget/BPW_EndGame.BPW_EndGame_C" null true))
      (`UserWidget.AddToViewport` _returnvalue 0)
      (set `PlayerController.bShowMouseCursor` true (`GameplayStatics.GetPlayerController` 0)))))

(fn `NextPhaseStart`
  (params (CurrentPhase :type Integer))
  (bind _outactors (`GameplayStatics.GetAllActorsOfClass` "/Game/Blueprint/EnemyCharacter/BP_CharacterEnemy_Base.BP_CharacterEnemy_Base_C"))
  (for _array_element _outactors
    (if (not (`/Game/Blueprint/EnemyCharacter/BP_CharacterEnemy_Base.bIsDead` _array_element))
      (`/Game/Blueprint/BP_KillScoreComponent.Destroy` (`/Game/Blueprint/EnemyCharacter/BP_CharacterEnemy_Base.BP_KillScoreComponent` _array_element)))))

(fn `TryRespawnEnemy`
  (locals (CurrentPoint :type "/Game/Blueprint/EnemySpawner/EnemySpawn Object Reference"))
  (bind _asbp_game_state (cast `/Game/Blueprint/Game/BP_GameState` (`GameplayStatics.GetGameState`)))
  (bind _valid (`/Game/Blueprint/Game/BP_GameState.CheckEnemyForPhase` _asbp_game_state))
  (if _valid
    (bind _returnvalue (select `int` (`/Game/Blueprint/Game/BP_GameState.CurrentPhase` _asbp_game_state) :`0` (`self.SpawnPointPhase1`) :`1` (`self.SpawnPointPhase2`) :`2` (`self.SpawnPointPhase3`) :`3` (`self.SpawnPointPhase4`) :`4` (`self.SpawnPointPhase5`)))
    (bind _output_get (set `local.CurrentPoint` (`|GetArrayItem` _returnvalue (`KismetMathLibrary.RandomIntegerInRange` 0 (- (`KismetArrayLibrary.Array_Length` _returnvalue) 1)))))
    (if (`/Game/Blueprint/EnemySpawner/EnemySpawn.bIsPoint` _output_get)
      (bind _returnvalue_2 (`self.K2_GetActorLocation` _output_get))
      (`|SpawnActorFromClass` "/Game/Blueprint/EnemyCharacter/BP_CharacterEnemy_Base.BP_CharacterEnemy_Base_C" (`KismetMathLibrary.Conv_VectorToTransform` _returnvalue_2) "AdjustIfPossibleButAlwaysSpawn" "OverrideRootScale" null null)
      (else
        (`|SpawnActorFromClass` "/Game/Blueprint/EnemyCharacter/BP_CharacterEnemy_Base.BP_CharacterEnemy_Base_C" (`KismetMathLibrary.Conv_VectorToTransform` (`KismetMathLibrary.RandomPointInBoundingBox` _returnvalue_2 (`BoxComponent.BoxExtent` (`/Game/Blueprint/EnemySpawner/EnemySpawn.Box` _output_get)))) "AdjustIfPossibleButAlwaysSpawn" "OverrideRootScale" null null)))
    (`/Game/Blueprint/Game/BP_GameState.IncrementEnemy` _asbp_game_state 1)))

(fn `TryToRespawnPlayer`
  (returns (Success :type Boolean))
  (bind _returnvalue (`GameplayStatics.GetPlayerController` 0))
  (bind _asbp_game_state (cast `/Game/Blueprint/Game/BP_GameState` (`GameplayStatics.GetGameState`)))
  (bind (_success _currentphase) (`/Game/Blueprint/Game/BP_GameState.CanPlayerRespawn` _asbp_game_state))
  (if _success
    (`self.RestartPlayerAtPlayerStart` _returnvalue (`self.K2_FindPlayerStart` _returnvalue (select `int` _currentphase :`0` "Phase0" :`1` "Phase1" :`2` "Phase2" :`3` "Phase3" :`4` "Phase4")))
    (return true)
    (else
      (return _success))))

(fn `UserConstructionScript`)