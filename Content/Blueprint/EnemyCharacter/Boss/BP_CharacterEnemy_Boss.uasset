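; BP_CharacterEnemy_Boss is a boss enemy character that carries a rocket turret.
; On BeginPlay it runs the parent logic, spawns a BP_TurretRocketBoss owned by itself at the mesh's RocketSocket, and snaps it onto that socket.
; It also prints the socket location as debug output; Tick is empty and the construction script only calls the parent.
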(event `self.ReceiveBeginPlay`
  (bind _mesh (`self.Mesh`))
  (bind _returnvalue (`SceneComponent.GetSocketLocation` _mesh "RocketSocket"))
  (`parent.ReceiveBeginPlay`)
  (`KismetSystemLibrary.PrintString` (`KismetStringLibrary.Conv_VectorToString` _returnvalue))
  (bind _returnvalue_2 (`|SpawnActorFromClass` "/Game/Blueprint/EnemyCharacter/Boss/Turret/BP_TurretRocketBoss.BP_TurretRocketBoss_C" (`KismetMathLibrary.Conv_VectorToTransform` _returnvalue) "AlwaysSpawn" "OverrideRootScale" self null))
  (`SceneComponent.K2_AttachToComponent` (`Actor.RootComponent` _returnvalue_2) _mesh "RocketSocket" "SnapToTarget" "SnapToTarget" "SnapToTarget" true))

(event `self.ReceiveTick`
  (params (DeltaSeconds :type "Float (single-precision)")))

(fn `UserConstructionScript`
  (`parent.UserConstructionScript`))